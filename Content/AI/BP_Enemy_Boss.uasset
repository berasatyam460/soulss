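; Boss enemy Blueprint that shows a boss health bar when the player character enters its trigger area.
; On overlap it creates and displays a WBP_BossHealth widget, waits a tick, then passes the bar to the BPCStat component; each qualifying overlap creates a new widget.
; BeginPlay runs the parent logic and caches the sword trace start and end world locations once.
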(event OnComponentBeginOverlap(Boss_triggerArea)
  (params (OverlappedComponent :type Primitive%20Component%20Object%20Reference) (OtherActor :type Actor%20Object%20Reference) (OtherComp :type Primitive%20Component%20Object%20Reference) (OtherBodyIndex :type Integer) (bFromSweep :type Boolean) (SweepResult :type Hit%20Result%20Structure%20%28by%20ref%29))
  (Utilities|Casting|CastToBP_ThirdPersonCharacter OtherActor)
  (bind _returnvalue (UserInterface|CreateWidget "/Game/UI/WBP_BossHealth.WBP_BossHealth_C"))
  (bind _output_get (Variables|Default|SetWBP_BossHUD _returnvalue))
  (UserInterface|Viewport|AddtoViewport _output_get 0)
  (Utilities|FlowControl|DelayUntilNextTick)
  (Default|SetHealthPriogressBar (Variables|Default|GetBPC_Stat) (Variables|/Game/UI/WBP_BossHealth.WBP_BossHealth_C|GetHealthBar (Variables|Default|GetWBP_BossHUD))))

(event EventBeginPlay
  (|CallParentFunction)
  (Variables|Default|SetStartBossSwordTrace_V (Transformation|GetWorldLocation (Variables|Default|GetStartBossSwordTrace_0)))
  (Variables|Default|SetEndBossSwordTrace_V (Transformation|GetWorldLocation (Variables|Default|GetEndBossSwordTrace_0))))

(fn ConstructionScript
  (|CallParentFunction))