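; BP_PatrolRoute is an AI patrol path that uses a spline's points as waypoints.
; An increment event steps the current point index by a direction value, reversing it at the first and last points for a back-and-forth route.
; A helper function returns the world location of the current spline point.
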(event Custom|IncreamentsPatrolRoutes
  (bind _output_get (Variables|Default|SetPatrolPointIndex (+ (Variables|Default|GetPatrolPointIndex) (Variables|Default|GetDirection))))
  (if (== _output_get (- (Spline|GetNumberOfSplinePoints (Variables|Default|GetPatrolRoutes)) 1))
    (Variables|Default|SetDirection -1)
    (elif (== (Variables|Default|GetPatrolPointIndex) 0)
      (Variables|Default|SetDirection 1))))

(fn ConstructionScript)

(fn SpinePointasWorldPos
  (return (Spline|GetLocationatSplinePoint (Variables|Default|GetPatrolRoutes) (Variables|Default|GetPatrolPointIndex) "World")))