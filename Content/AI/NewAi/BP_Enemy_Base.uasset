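; Base sword-wielding enemy character with a floating health bar, lock-on widget and patrol route, driven by AIC_Enemy_Base.
; Health, damage and healing forward to BPCDAmageSystem, whose hit response freezes the AI, plays a reaction montage, then resumes attacking.
; Montages handle attacks and spawn or destroy the sword on draw or sheathe.
; A looping timer sphere-traces sword swings, damaging the player found by class rather than the hit actor.
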(event Custom|WiledSwrds
  ;[0 0 0] WeildSword
  (bind _notifyname (Animation|Montage|PlayMontage (Variables|Character|GetMesh) "/Game/Mixamo/NewAnim/SheathingSword_UE_Montage.SheathingSword_UE_Montage" -1.0 1.67 "Default")
    (:OnCompleted
      (Default|CallOnWeildShield))
    (:OnNotifyBegin
      (switch name _notifyname
        (:EquipWeapon
          (bind _returnvalue (Game|SpawnActorfromClass "/Game/Weapons/BP_Sword.BP_Sword_C" (Transformation|GetActorTransform) "Undefined" "MultiplyWithRoot" 0 0))
          (Variables|Default|SetSwordActor _returnvalue)
          (Transformation|AttachComponentToComponent _returnvalue (Variables|Character|GetMesh) "Equip_Sword" "SnapToTarget" "SnapToTarget" "SnapToTarget" true)
          (Variables|Default|SetIsWeldingSword true))))))

(event Custom|ShealthSword
  ;[0 0 0] Shelathsword
  (bind _notifyname (Animation|Montage|PlayMontage (Variables|Character|GetMesh) "/Game/Mixamo/NewAnim/SheathingSword_UE_Montage.SheathingSword_UE_Montage" 1.0 0.0 "Default")
    (:OnCompleted
      (Default|CallOnShealthSword))
    (:OnNotifyBegin
      (switch name _notifyname
        (:EquipWeapon
          (Actor|DestroyActor (Variables|Default|GetSwordActor))
          (Variables|Default|SetIsWeldingSword false))))))

(event Custom|DamageTrace
  ;[0 0 0] Sword Traces
  (bind _isdead_ (CallFunction|IsDead))
  (if (not _isdead_)
    (bind (_outhit _returnvalue) (Collision|SphereTraceForObjects (Transformation|GetWorldLocation (Variables|Default|GetStartArrow)) (Transformation|GetWorldLocation (Variables|Default|GetEndArrow)) (Variables|Default|GetSwordAttackRadius) (Utilities|Array|MakeArray "ObjectTypeQuery3") false 0 "ForOneFrame"))
    (if _returnvalue
      (Utilities|FlowControl|DoOnce false :!label _label
        (:Completed
          (bind _returnvalue_2 (Actor|GetActorOfClass "/Game/ThirdPerson/Blueprints/BP_ThirdPersonCharacter.BP_ThirdPersonCharacter_C"))
          (Default|TakeDamage _returnvalue_2 (Utilities|Struct|MakeS_DamageInfo 1.0 "NewEnumerator1" "NewEnumerator0" false false true))
          (Camera|PlayWorldCameraShake "/Game/Bluprints/BS_CameraShake.BS_CameraShake_C" (.Location (Collision|BreakHitResult _outhit)) 0.0 2e+03)
          (Utilities|FlowControl|Delay 0.3)
          (goto _label Reset))))))

(event Custom|HitResponse
  (params (DamageRespose :type E_ResposeType%20Enum :default "NewEnumerator0"))
  (Components|Movement|StopMovementImmediately (Variables|Character|GetCharacterMovement))
  (Default|SetStateasFrozen (Variables|Default|GetAIC%20Enemy%20Base%20Controller))
  (switch Utilities|FlowControl|Switch|SwitchonE_ResposeType DamageRespose
    (:NewEnumerator1
      (Animation|Montage|PlayMontage (Variables|Character|GetMesh) (Variables|Default|GetMontageForHitReaction)
        (:OnCompleted
          _)
        (:OnInterrupted
          _))
      (Default|SetStateasAttacking (Variables|Default|GetAIC%20Enemy%20Base%20Controller) 0 true))))

(event Custom|Attack
  ;[0 0 0] Attack
  (Animation|Montage|PlayMontage (Variables|Character|GetMesh) "/Game/Characters/Souls/Combat/SwordAttackCombo_Montage.SwordAttackCombo_Montage"
    (:then
      (Variables|/Game/DAmageSystem/BPC_DAmageSystem.BPC_DAmageSystem_C|SetIsIntruptabl;e (Variables|Default|GetBPC_DAmageSystem) false))
    (:OnCompleted
      (Default|CallOnAttackEnd :!label _label))
    (:OnInterrupted
      (goto _label))))

(event EventToggleLockonWidget
  (params (Visible :type Boolean))
  (Rendering|SetVisibility (Variables|Default|GetLockOnWidget) Visible false))

(event EventBeginSwordTrace
  ;[0 0 0] Sword Traces
  (bind _returnvalue (Utilities|Time|SetTimerbyEvent (delegate Custom|DamageTrace) 0.01 true)))

(event EventEndSwordTrace
  ;[0 0 0] Sword Traces
  (if (Utilities|Time|IsValidTimerHandle (stale EventBeginSwordTrace _returnvalue))
    (Utilities|Time|ClearandInvalidateTimerbyHandle (stale EventBeginSwordTrace _returnvalue))))

(event EventBeginPlay
  (bind _self self)
  (bind _bpc_damagesystem (Variables|Default|GetBPC_DAmageSystem))
  (Utilities|FlowControl|Delay 1.0)
  (bind _returnvalue (UserInterface|CreateWidget "/Game/UI/WBP_EnemyHealth.WBP_EnemyHealth_C" 0 _self _self))
  (UserInterface|SetWidget (Variables|Default|GetW_HealthBar) _returnvalue)
  (Default|SetHealthPriogressBar _bpc_damagesystem (Variables|/Game/UI/WBP_EnemyHealth.WBP_EnemyHealth_C|GetHealthBar _returnvalue) (Variables|/Game/UI/WBP_EnemyHealth.WBP_EnemyHealth_C|GetHealthBarAnim _returnvalue))
  (Utilities|FlowControl|Delay 1.0)
  (bind _asaic_enemy_base (Utilities|Casting|CastToAIC_Enemy_Base (AI|GetAIController self)))
  (Variables|Default|SetAIC%20Enemy%20Base%20Controller _asaic_enemy_base)
  (EventDispatchers|AssignOnDamageRespose _bpc_damagesystem (EventDispatchers|CreateEvent :!event Custom|HitResponse)))

(fn ConstructionScript)

(fn GetDirection
  (params (InputAction :type Input%20Action%20Object%20Reference))
  (bind _returnvalue (Class|EnhancedInputSubsystemInterface|QueryKeysMappedtoAction(Message) (PlayerController|LocalPlayerSubsystems|GetEnhancedInputLocalPlayerSubsystem (Game|GetPlayerController 0)) InputAction))
  (for _array_element _returnvalue
    (if (Game|Player|IsInputKeyDown (Game|GetPlayerController 0) _array_element)
      (return _array_element))))

(fn GetPatrolRoutes
  (return (Variables|AI|GetPatrolRoutes)))

(fn GetCurrentHealth
  (return (Variables|/Game/DAmageSystem/BPC_DAmageSystem.BPC_DAmageSystem_C|GetHealth (Variables|Default|GetBPC_DAmageSystem))))

(fn GetIdealRange
  (return 1.5e+02 3.5e+02))

(fn GetMaxHealth
  (return (Variables|/Game/DAmageSystem/BPC_DAmageSystem.BPC_DAmageSystem_C|GetMaxHealth (Variables|Default|GetBPC_DAmageSystem))))

(fn GetPatrolPoints
  (return (Variables|AI|GetPatrolRoutes)))

(fn Heal
  (params (HealAmount :type Float%20%28double-precision%29))
  (bind _newhealth (Default|Heal (Variables|Default|GetBPC_DAmageSystem) HealAmount))
  (return _newhealth))

(fn IsDead
  (return (Variables|/Game/DAmageSystem/BPC_DAmageSystem.BPC_DAmageSystem_C|GetISDead (Variables|Default|GetBPC_DAmageSystem))))

(fn SetMoveSpeed
  (params (Speed :type E_MovementSpeed%20Enum :default "NewEnumerator0"))
  (bind _output_get (Variables|/Script/Engine.CharacterMovementComponent|SetMaxWalkSpeed (Variables|Character|GetCharacterMovement) (Utilities|Select :Index Speed :NewEnumerator0 0.0 :NewEnumerator1 1e+02 :NewEnumerator2 3e+02 :NewEnumerator3 5e+02)))
  (return _output_get))

(fn TakeDamage
  (params (DamageInfo :type S%20Damage%20Info%20Structure))
  (bind _wasdamaged (Default|TakeDamage (Variables|Default|GetBPC_DAmageSystem) DamageInfo))
  (return _wasdamaged))