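; Actor component that manages an actor's health, stamina, damage, blocking and death.
; TakeDamage uses CanBeDamaged to filter dead, invincible or blocking states, then fires blocked, death or response dispatchers; interruptible hits subtract damage twice.
; IncreaseValue clamps stats and updates bars, with a timer easing the health background bar.
; The RegainStamina timer actually adds Health, and the Stamina branch ignores its Amount.
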(event Custom|Die
  (Class|BPIDamage|Die(Message) (Components|GetOwner)))

(event Custom|Set%20Health%20Priogress%20Bar
  (params (Health%20Progress%20Bar :type Progress%20Bar%20Object%20Reference) (HealthProgressBarBG :type Progress%20Bar%20Object%20Reference))
  (Variables|Default|SetHealth%20Progress%20Bar Health%20Progress%20Bar)
  (Variables|Default|SetHealth%20Progress%20Bar%20BG HealthProgressBarBG))

(event Custom|Set%20stamina%20Progress%20Bar
  (params (Health%20StaminaBar :type Progress%20Bar%20Object%20Reference))
  (Variables|Default|SetHealth%20StaminaBar Health%20StaminaBar))

(event Custom|RegainStamina
  (if (Variables|Default|GetRegain%20Stamina?)
    (CallFunction|IncreaseValue "NewEnumerator0" 0.5)))

(event Custom|AnimateHealthbarBG
  (Utilities|Time|ClearandInvalidateTimerbyHandle (Variables|Default|GetHealthTimer))
  (Variables|Default|GetHealth%20Progress%20Bar%20BG
    (:then
      (bind _returnvalue (Utilities|Time|SetTimerbyEvent (delegate Custom|op) 0.03 true))
      (Variables|Default|SetHealthTimer _returnvalue))
    (:else)))

(event Custom|op
  (if (Math|Float|NearlyEqual(Float) (Variables|/Script/UMG.ProgressBar|GetPercent (Variables|Default|GetHealth%20Progress%20Bar%20BG)) (Variables|/Script/UMG.ProgressBar|GetPercent (Variables|Default|GetHealth%20Progress%20Bar)) 1.0)
    (Progress|SetPercent (Variables|Default|GetHealth%20Progress%20Bar%20BG) (Math|Interpolation|FInterpTo (Variables|/Script/UMG.ProgressBar|GetPercent (Variables|Default|GetHealth%20Progress%20Bar%20BG)) (Variables|/Script/UMG.ProgressBar|GetPercent (Variables|Default|GetHealth%20Progress%20Bar)) 1.0 0.1))
    (else
      (Progress|SetPercent (Variables|Default|GetHealth%20Progress%20Bar%20BG) (Variables|/Script/UMG.ProgressBar|GetPercent (Variables|Default|GetHealth%20Progress%20Bar)))
      (Utilities|Time|ClearandInvalidateTimerbyHandle (Variables|Default|GetHealthTimer)))))

(event EventBeginPlay
  (Utilities|Time|SetTimerbyEvent (delegate Custom|RegainStamina) 0.01 true))

(fn Heal
  (params (HealAmount :type Float%20%28double-precision%29))
  (if (not (Variables|Default|GetISDead))
    (bind _output_get (Variables|Default|SetHealth (Math|Float|Clamp(Float) (+ HealAmount (Variables|Default|GetHealth)) 0.0 (Variables|Default|GetMaxHealth))))
    (return _output_get)))

(fn TakeDamage
  (params (DamageInfo :type S%20Damage%20Info%20Structure))
  (bind (_amount _damagetype _damagerespose _shoulddamageinvinsicle _canbeblocked _shouldforceinterrupt _canbeparry) (Utilities|Struct|BreakS_DamageInfo DamageInfo))
  (Utilities|CanbeDamaged _shoulddamageinvinsicle _canbeblocked
    (:BlockDamage
      (Development|PrintString "Blocked")
      (Default|CallOnBlocked _canbeparry)
      (return false))
    (:DoDamage
      (bind _output_get (Variables|Default|SetHealth (- (Variables|Default|GetHealth) _amount)))
      (if (<= _output_get 0.0)
        (Variables|Default|SetISDead true)
        (Default|CallOnDead)
        (Development|PrintString "D")
        (return true)
        (elif (or (Variables|Default|GetIsIntruptabl;e) _shouldforceinterrupt)
          (Default|CallOnDamageRespose _damagerespose)
          (Development|PrintString "Get damage")
          (CallFunction|IncreaseValue "NewEnumerator0" (* _amount -1.0))
          (return true))))
    (:NoDamage
      (return false))))

(fn IncreaseValue
  (params (Stat :type E_Stat%20Enum :default "NewEnumerator0") (Amount :type Float%20%28double-precision%29))
  (switch Utilities|FlowControl|Switch|SwitchonE_Stat Stat
    (:NewEnumerator0
      (Variables|Default|Sethealth (Math|Float|Clamp(Float) (+ (Variables|Default|Gethealth) Amount) 0.0 (Variables|Default|GetMaxHealth)))
      (Utilities|FlowControl|Sequence
        (:then_0
          (if (<= (Variables|Default|Gethealth) 0.0)
            (CallFunction|Die)))
        (:then_1
          (bind _health_progress_bar (Variables|Default|GetHealth%20Progress%20Bar)
            (:then
              (Progress|SetPercent _health_progress_bar (/ (Variables|Default|Gethealth) (Variables|Default|GetMaxHealth)))
              (CallFunction|AnimateHealthbarBG))
            (:else)))))
    (:NewEnumerator1
      (Variables|Default|SetStamina (Math|Float|Clamp(Float) (+ (Variables|Default|GetStamina) 0.0) 0.0 (Variables|Default|GetMaxStamina)))
      (bind _health_staminabar (Variables|Default|GetHealth%20StaminaBar)
        (:then
          (Progress|SetPercent _health_staminabar (/ (Variables|Default|GetStamina) (Variables|Default|GetMaxStamina))))
        (:else)))))